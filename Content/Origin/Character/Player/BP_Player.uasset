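; BP_Player is the player character Blueprint, handling attack, sprint and state changes through networked event chains.
; Call events forward to server events, and attacks continue to a multicast that plays AM_Attack only in the Movable state, then marks the character Attacking.
; A combo flag selects the Attack2 montage section over Attack1 and is cleared on use.
; Sprint toggles max walk speed via a server-side FlipFlop.
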(event `CallStateChange`
  (params (State :type "/Game/Origin/Data/Enum/E_CharacterState Enum" :default "NewEnumerator0"))
  (`self.StateChangeOnServer` State))

(event `StateChangeOnServer`
  (params (State :type "/Game/Origin/Data/Enum/E_CharacterState Enum" :default "NewEnumerator0"))
  (set `self.CurrentState` State))

(event `CallAttackInput`
  (`self.AttackOnServer`))

(event `AttackOnServer`
  (`self.AttackMulticast`))

(event `AttackMulticast`
  (switch `/Game/Origin/Data/Enum/E_CharacterState` (`self.CurrentState`)
    (:`NewEnumerator2`
      (set `self.CurrentState` "NewEnumerator0")
      (if (`self.bIsComboInputOn`)
        (`self.PlayAnimMontage` "/Game/Origin/Animation/AM_Attack.AM_Attack" 1.0 "Attack2")
        (set `self.bIsComboInputOn` false)
        (else
          (`self.PlayAnimMontage` "/Game/Origin/Animation/AM_Attack.AM_Attack" 1.0 "Attack1"))))))

(event `CallSprintInput`
  (`self.SprintOnServer`))

(event `SprintOnServer`
  (bind _charactermovement (`self.CharacterMovement`))
  (`/Engine/EditorBlueprintResources/StandardMacros.FlipFlop`
    (:`A`
      (set `CharacterMovementComponent.MaxWalkSpeed` 675.0 _charactermovement))
    (:`B`
      (set `CharacterMovementComponent.MaxWalkSpeed` 500.0 _charactermovement))))

(fn `UserConstructionScript`
  (`parent.UserConstructionScript`))