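; Game mode that periodically spawns falling arrow hazards around a target point in the level.
; On BeginPlay it starts a looping timer for SpawnStones and caches a TargetPoint actor.
; Each tick of the timer spawns a scaled-up BP_FallingArrow at a random point in a box centered on that target, with randomized X and Y extents.
; A short lifespan on each arrow handles cleanup.
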(event `self.ReceiveBeginPlay`
  (`KismetSystemLibrary.K2_SetTimerDelegate` (delegate `SpawnStones`) 2.0 true)
  (bind _returnvalue (`GameplayStatics.GetActorOfClass` "/Script/Engine.TargetPoint"))
  (set `self.TargetPointRef` _returnvalue))

(event `SpawnStones`
  (bind _returnvalue (`|SpawnActorFromClass` "/Game/Origin/OtherActor/BP_FallingArrow.BP_FallingArrow_C" (`KismetMathLibrary.MakeTransform` (`KismetMathLibrary.RandomPointInBoundingBox` (`self.K2_GetActorLocation` (`self.TargetPointRef`)) (`KismetMathLibrary.MakeVector` (`KismetMathLibrary.RandomFloatInRange` 0.0 1000.0) (`KismetMathLibrary.RandomFloatInRange` 0.0 1000.0))) (struct) (2.0 2.0 2.0)) "Undefined" "MultiplyWithRoot" null null))
  (`self.SetLifeSpan` _returnvalue 8.0))

(fn `UserConstructionScript`)